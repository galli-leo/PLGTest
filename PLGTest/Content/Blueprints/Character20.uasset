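; Character Blueprint that lets the player rotate the camera around the character by holding keys.
; Holding E or Q opens a gate on Tick, which yaws the CameraBoom in opposite directions at a fixed rate scaled by delta time.
; Pitch and roll stay unchanged, and releasing a key closes its gate to stop that rotation.
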(event EventTick
  (params (DeltaSeconds :type Float%20%28single-precision%29))
  (bind _cameraboom (Variables|Default|GetCameraBoom))
  (bind _cameraboom_2 (Variables|Default|GetCameraBoom))
  (bind _relativerotation (Variables|/Script/Engine.SceneComponent|GetRelativeRotation _cameraboom))
  (bind _relativerotation_2 (Variables|/Script/Engine.SceneComponent|GetRelativeRotation _cameraboom_2))
  (bind (_pitch _yaw _roll) (Class|KismetMathLibrary|BreakRot _relativerotation_2))
  (bind (_pitch_2 _yaw_2 _roll_2) (Class|KismetMathLibrary|BreakRot _relativerotation))
  (Utilities|FlowControl|Sequence
    (:then_0
      (Utilities|FlowControl|Gate true
        (:Exit
          (Transformation|SetRelativeRotation _cameraboom_2 (Class|KismetMathLibrary|MakeRot _pitch (+ _yaw (* DeltaSeconds 1.5e+02)) _roll) false))))
    (:then_1
      (Utilities|FlowControl|Gate true
        (:Exit
          (Transformation|SetRelativeRotation _cameraboom (Class|KismetMathLibrary|MakeRot _pitch_2 (+ _yaw_2 (* DeltaSeconds -1.5e+02)) _roll_2) false))))))

(event Input|KeyboardEvents|Q
  (bind _cameraboom (Variables|Default|GetCameraBoom))
  (bind _relativerotation (Variables|/Script/Engine.SceneComponent|GetRelativeRotation _cameraboom))
  (bind (_pitch _yaw _roll) (Class|KismetMathLibrary|BreakRot _relativerotation))
  (:Pressed
    (Utilities|FlowControl|Gate true) ; enters at Open
  )
  (:Released
    (Utilities|FlowControl|Gate true) ; enters at Close
  ))

(event Input|KeyboardEvents|E
  (bind _cameraboom (Variables|Default|GetCameraBoom))
  (bind _relativerotation (Variables|/Script/Engine.SceneComponent|GetRelativeRotation _cameraboom))
  (bind (_pitch _yaw _roll) (Class|KismetMathLibrary|BreakRot _relativerotation))
  (:Pressed
    (Utilities|FlowControl|Gate true) ; enters at Open
  )
  (:Released
    (Utilities|FlowControl|Gate true) ; enters at Close
  ))

(fn ConstructionScript)