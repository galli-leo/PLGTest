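; Wall light that, on a rare random roll each tick, plays a flickering electrical fault with spark effects.
; The Spark timeline drives spotlight intensity and the "Light" parameter of a dynamic material created on the mesh in the construction script.
; A parallel chain of delays fires two particle systems in staggered bursts.
; A particle toggle inside the timeline update sits behind a constant comparison that never passes.
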(event EventTick
  (params (DeltaSeconds :type Float%20%28single-precision%29))
  (bind _particlesystem1 (Variables|Default|GetParticleSystem1))
  (bind _particlesystem2 (Variables|Default|GetParticleSystem2))
  (bind _particlesystem1_2 (Variables|Default|GetParticleSystem1))
  (bind _particlesystem2_2 (Variables|Default|GetParticleSystem2))
  (Math|Integer|CompareInt (Math|Random|RandomIntegerinRange 0 10000) 0
    (:==
      (Utilities|FlowControl|Sequence
        (:then_0
          (bind _bright (Timeline|spark Play)
            (:Update
              (Rendering|Components|Light|SetIntensity (Variables|Default|GetSpotLight2) (* _bright 9e+02))
              (Rendering|Material|SetScalarParameterValue (Variables|Default|GetMaterialInst) "Light" _bright :!class /Script/Engine.MaterialInstanceDynamic)
              (Math|Float|CompareFloat 1.0 0.0
                (:<
                  (if (Components|Activation|IsActive _particlesystem1_2)
                    (Components|Activation|Activate _particlesystem2_2 false)
                    (Utilities|FlowControl|Delay 0 0.8)
                    (Components|Activation|Deactivate _particlesystem2_2)
                    (else
                      (Components|Activation|Activate _particlesystem1_2 false)
                      (Utilities|FlowControl|Delay 0 0.8)
                      (Components|Activation|Deactivate _particlesystem1_2))))))))
        (:then_1
          (Utilities|FlowControl|Delay 0 0.05)
          (Components|Activation|Activate _particlesystem1 false)
          (Utilities|FlowControl|Delay 0 0.9)
          (Components|Activation|Deactivate _particlesystem1)
          (Utilities|FlowControl|Delay 0 0.65)
          (Components|Activation|Activate _particlesystem1 false)
          (Utilities|FlowControl|Sequence
            (:then_0
              (Utilities|FlowControl|Delay 0 0.9)
              (Components|Activation|Deactivate _particlesystem1)
              (Utilities|FlowControl|Delay 0 0.65))
            (:then_1
              (Utilities|FlowControl|Delay 0 0.55)
              (Components|Activation|Activate _particlesystem2 false)
              (Utilities|FlowControl|Delay 0 0.9)
              (Components|Activation|Deactivate _particlesystem2))))))))

(fn ConstructionScript
  (bind _staticmesh2 (Variables|Default|GetStaticMesh2))
  (bind _returnvalue (Rendering|Material|CreateDynamicMaterialInstance (Rendering|Material|GetMaterial _staticmesh2 0) "/Game/Props/02_-_Default.02_-_Default" :!class /Script/Engine.KismetMaterialLibrary))
  (Variables|Default|SetMaterialInst _returnvalue)
  (Rendering|Material|SetMaterial _staticmesh2 0 (Variables|Default|GetMaterialInst)))